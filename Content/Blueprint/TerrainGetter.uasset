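; TerrainGetter is a component that reports which terrain its owning actor stands on.
; GetTerrain runs a zero-radius sphere overlap at the owner's location, filtered to WorldDynamic BaseTerrain actors, and takes the first hit.
; It returns that actor's class and terrain name, or prints a message and falls back to Plains when the cast fails.
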(fn `getTerrain`
  (returns (currentTerrain :type "/Game/Blueprint/Terrain/BaseTerrain Class Reference") (currentTerrainName :type String))
  (bind _outactors (`KismetSystemLibrary.SphereOverlapActors` (`Actor.K2_GetActorLocation` (`self.GetOwner`)) 0.0 (`|MakeArray` "ObjectTypeQuery2" :!type "EObjectTypeQuery Enum") "/Game/Blueprint/Terrain/BaseTerrain.BaseTerrain_C"))
  (bind _asbase_terrain (cast `/Game/Blueprint/Terrain/BaseTerrain` (`|GetArrayItem` _outactors))
    (:`then`
      (return (`GameplayStatics.GetObjectClass` _asbase_terrain) (`/Game/Blueprint/Terrain/BaseTerrain.terrainName` _asbase_terrain)))
    (:`CastFailed`
      (`KismetSystemLibrary.PrintString` "No terrain found. Defaulting to Plains.")
      (return "/Game/Blueprint/Terrain/Plains.Plains_C" "Plains"))))