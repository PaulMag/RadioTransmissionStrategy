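; RTS game mode that sets up the HUD, mouse control and actor references when play begins.
; BeginPlay creates the GeneralHud widget, adds it to the viewport, and enables the cursor and click events for the first player controller.
; It caches all Token, Unit and City actors in arrays, then cross-links tokens and units by array index, relying on matching order and count.
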(event `self.ReceiveBeginPlay`
  (bind _returnvalue (`GameplayStatics.GetPlayerController` 0))
  (`|ExecutionSequence`
    (:`then_0`
      ;[1 1 1] Initialize HUD
      (bind _returnvalue_2 (`|CreateWidget` "/Game/Blueprint/GeneralHud.GeneralHud_C"))
      (bind _output_get (set `self.generalHUD` _returnvalue_2))
      (`UserWidget.AddToViewport` _output_get 0))
    (:`then_1`
      ;[1 1 1] Enable mouse control
      (set `PlayerController.bShowMouseCursor` true _returnvalue)
      (set `PlayerController.bEnableClickEvents` true _returnvalue)
      ;[1 1 1] Fill token, unit, city arrays
      (bind _outactors (`GameplayStatics.GetAllActorsOfClass` "/Game/Blueprint/Token.Token_C"))
      (set `self.tokens` _outactors)
      (bind _outactors_2 (`GameplayStatics.GetAllActorsOfClass` "/Game/Blueprint/Unit.Unit_C"))
      (set `self.units` _outactors_2)
      (bind _outactors_3 (`GameplayStatics.GetAllActorsOfClass` "/Game/Blueprint/City.City_C"))
      (set `self.cities` _outactors_3)
      ;[1 1 1] Pair each unit with a token
      (for (_array_element _array_index) (`self.tokens`)
        (bind _output (`|GetArrayItem` (`self.units`) _array_index))
        (set `/Game/Blueprint/Token.unit` _output _array_element)
        (set `/Game/Blueprint/Unit.token` (`|GetArrayItem` (`self.tokens`) _array_index) _output)))))

(event `self.ReceiveTick`
  (params (DeltaSeconds :type "Float (single-precision)")))

(fn `UserConstructionScript`)