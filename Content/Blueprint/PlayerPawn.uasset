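; Player pawn that lets the player select, drag and issue move orders to tokens on a table.
; Left click traces under the cursor to select a Token, and while held, Tick moves it to the cursor's hit point on a Table at zero height.
; Key 2 arms a move command, and the next right click writes the traced cursor location to the selected token's Unit.
; Token picking and surface placement use separate trace channels.
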(event `Key|LeftMouseButton`
  (params (Key :type "Key Structure"))
  ;[1 1 1] Select a token and enter dragging mode
  (:`Pressed`
    (bind _astoken (cast `/Game/Blueprint/Token` (`.HitActor` (`GameplayStatics.BreakHitResult` (`PlayerController.GetHitResultUnderCursorByChannel` (`GameplayStatics.GetPlayerController` 0) "TraceTypeQuery4" true))))
      (:`then`
        (set `self.selectedToken` _astoken)
        (set `self.dragging` true))
      (:`CastFailed`
        (`KismetSystemLibrary.PrintString` "Casting failed!"))))
  (:`Released`
    (set `self.dragging` false)))

(event `self.ReceiveTick`
  (params (DeltaSeconds :type "Float (single-precision)"))
  (bind (_bblockinghit _binitialoverlap _time _distance _location _impactpoint _normal _impactnormal _physmat _hitactor) (`GameplayStatics.BreakHitResult` (`PlayerController.GetHitResultUnderCursorByChannel` (`GameplayStatics.GetPlayerController` 0) "TraceTypeQuery3" true)))
  ;[1 1 1] Drag token
  (if (`self.dragging`)
    (if (== (`GameplayStatics.GetObjectClass` _hitactor) "/Game/Blueprint/Table.Table_C")
      (`self.K2_SetActorLocation` (`self.selectedToken`) (`KismetMathLibrary.MakeVector` (.x _location) (.y _location)) false false))))

(event `Key|Two`
  (params (Key :type "Key Structure"))
  ;[1 1 1] Issue move command
  (:`Pressed`
    (set `self.moveCommand` true)))

(event `Key|RightMouseButton`
  (params (Key :type "Key Structure"))
  (bind (_hitresult _returnvalue) (`PlayerController.GetHitResultUnderCursorByChannel` (`GameplayStatics.GetPlayerController` 0) "TraceTypeQuery3" true))
  ;[1 1 1] Issue move command
  (:`Pressed`
    (if (`self.moveCommand`)
      (set `self.moveCommand` false)
      (if _returnvalue
        (set `/Game/Blueprint/Unit.moveCommand` (`.Location` (`GameplayStatics.BreakHitResult` _hitresult)) (`/Game/Blueprint/Token.unit` (`self.selectedToken`)))))))

(fn `UserConstructionScript`)