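; Token is a map piece actor that represents a Unit and its faction.
; On BeginPlay it hides its UI, spawns a Unit of UnitType at its location if none is set, and passes it the faction number.
; Units outside the player's faction start random targeting, while the player's have it deactivated.
; It then sets the Unit's faction color and picks its own mesh from a per-faction list.
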(event `self.ReceiveBeginPlay`
  (bind _randomtargetingcomponent (`/Game/Blueprint/Units/Unit.RandomTargetingComponent` (`self.unit`)))
  (`|ExecutionSequence`
    (:`then_0`
      (`SceneComponent.SetVisibility` (`self.UI`) false false))
    (:`then_1`
      ;[1 1 1] Spawn the Tokens corresponding Unit if one is not already set
      (`/Engine/EditorBlueprintResources/StandardMacros.IsValid` (`self.unit`) ; if is not null
        (:`Is Not Valid`
          (bind _returnvalue (`|SpawnActorFromClass` (`self.unitType`) (`KismetMathLibrary.Conv_VectorToTransform` (`self.K2_GetActorLocation` self)) "AlwaysSpawn" "OverrideRootScale" null null))
          (set `self.unit` _returnvalue))))
    (:`then_2`
      ;[1 1 1] Set Unit to correct faction. Faction depended stuff must happen after this.
      (set `BaseUnit.factionNumber` (`self.factionNumber`) (`self.unit`)))
    (:`then_3`
      ;[1 1 1] Set if Unit is AI controlled
      (if (!= (`/Game/Blueprint/PlayerPawn.factionNumber` (cast `/Game/Blueprint/PlayerPawn` (`GameplayStatics.GetPlayerPawn` 0) :!pure true)) (`self.factionNumber`))
        (`/Game/Blueprint/RandomTargetingComponent.start` _randomtargetingcomponent)
        (else
          (`ActorComponent.Deactivate` _randomtargetingcomponent))))
    (:`then_4`
      ;[1 1 1] Turn on mesh representing correct faction and turn of all others
      (`/Game/Blueprint/Units/Unit.setFactionColor` (`self.unit`)) ; Set faction color on the Unit's test sphere
      (`StaticMeshComponent.SetStaticMesh` (`self.tokenMesh`) (`|GetArrayItem` (`self.factionMeshes`) (`self.factionNumber`))))))

(fn `UserConstructionScript`)