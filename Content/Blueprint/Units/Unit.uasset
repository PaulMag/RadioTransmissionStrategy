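; RTS Unit actor that belongs to a faction, moves toward a move command and compiles text radio reports.
; Tick updates the strength widget and steps toward MoveCommand, line-tracing to follow landscape height.
; BeginPlay and terrain end-overlaps query TerrainGetter to scale base speed by terrain.
; MakeRadioReport describes position from the nearest Landmark, terrain, heading and enemies within vision range, using rounded distances and compass directions.
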(event `self.ReceiveActorBeginOverlap`
  (params (OtherActor :type "Actor Object Reference"))
  (bind _returnvalue (`GameplayStatics.GetObjectClass` OtherActor))
  ;[1 1 1] Adjust speed according to terrain
  (`parent.ReceiveActorBeginOverlap` OtherActor)
  (if (`KismetMathLibrary.ClassIsChildOf` _returnvalue "/Game/Blueprint/Terrain/BaseTerrain.BaseTerrain_C")
    (bind _asbase_terrain (castclass `/Game/Blueprint/Terrain/BaseTerrain` _returnvalue))
    (set `self.currentTerrain` _asbase_terrain)))

(event `self.ReceiveActorEndOverlap`
  (params (OtherActor :type "Actor Object Reference"))
  (`parent.ReceiveActorEndOverlap` OtherActor)
  (if (`KismetMathLibrary.ClassIsChildOf` (`GameplayStatics.GetObjectClass` OtherActor) "/Game/Blueprint/Terrain/BaseTerrain.BaseTerrain_C")
    ;[1 1 1] Adjust current speed based on terrain
    (bind (_currentterrain _currentterrainname) (`/Game/Blueprint/TerrainGetter.getTerrain` (`self.TerrainGetter`) :!label _label))
    (set `self.currentTerrain` _currentterrain)
    (set `self.currentTerrainName` _currentterrainname)
    (set `self.speedCurrent` (* (`BlueprintMapLibrary.Map_Find` (`self.terrainToSpeed`) (`self.currentTerrain`)) (`self.speedBase`)))))

(event `self.ReceiveBeginPlay`
  (`parent.ReceiveBeginPlay`)
  (`|ExecutionSequence`
    (:`then_0`
      (goto _label))
    (:`then_1`
      ;[1 1 1] Initial move command to self => do not move
      (set `self.moveCommand` (`self.K2_GetActorLocation`)))))

(event `setFactionColor`
  ;[1 1 1] Set faction color on the test sphere
  (`PrimitiveComponent.SetMaterial` (`self.unitBall`) 0 (`|GetArrayItem` (`self.factionColors`) (`self.factionNumber`))))

(event `self.ReceiveTick`
  (params (DeltaSeconds :type "Float (single-precision)"))
  (bind _returnvalue (`self.K2_GetActorLocation`))
  (`parent.ReceiveTick` DeltaSeconds)
  (`|ExecutionSequence`
    (:`then_0`
      ;[1 1 1] Set the strength widget to display the current hit points of this Unit
      (bind _asunit_strength_hud (cast `/Game/UI/UnitStrengthHUD` (`WidgetComponent.GetUserWidgetObject` (`self.strengthWidget`))))
      (set `/Game/UI/UnitStrengthHUD.strength` (`self.strength`) _asunit_strength_hud))
    (:`then_1`
      ;[1 1 1] Follow landscape (only cosmetic)
      (bind _outhit (`KismetSystemLibrary.LineTraceSingle` (+ _returnvalue (0.0 0.0 10.0)) (- _returnvalue (0.0 0.0 10.0)) "TraceTypeQuery3" true))
      ;[1 1 1] Move towards move command
      (`self.K2_SetActorLocation` (+ (* (`KismetMathLibrary.GetDirectionUnitVector` (`self.K2_GetActorLocation`) (`self.moveCommand`)) (* DeltaSeconds (`self.speedCurrent`))) (`self.K2_GetActorLocation`) (`KismetMathLibrary.MakeVector` 0.0 0.0 (- (.z (`.ImpactPoint` (`GameplayStatics.BreakHitResult` _outhit))) (.z _returnvalue))))))))

(fn `makeRadioReport`
  (locals (unitsObservedString :type String))
  (`|ExecutionSequence`
    (:`then_0`
      ;[1 1 1] Find closest Landmark
      (set `self.closestLandmarkDistance` 1000000.0)
      (bind _outactors (`GameplayStatics.GetAllActorsOfClass` "/Game/Blueprint/Landmark.Landmark_C"))
      (for _array_element _outactors
        (bind _returnvalue (`KismetMathLibrary.VSize` (- (`self.K2_GetActorLocation` _array_element) (`self.K2_GetActorLocation`))))
        (if (< _returnvalue (`self.closestLandmarkDistance`))
          (set `self.closestLandmark` _array_element)
          (set `self.closestLandmarkDistance` _returnvalue))))
    (:`then_1`
      ;[1 1 1] Find other units in vision
      (bind _asrtsgame_mode (cast `/Game/Blueprint/RTSGameMode` (`GameplayStatics.GetGameMode`)))
      (set `self.unitsInVision` (`|MakeSet`)) ; initialize empty set
      (for _array_element_2 (`/Game/Blueprint/RTSGameMode.units` _asrtsgame_mode)
        (if (!= (`self.factionNumber`) (`BaseUnit.factionNumber` _array_element_2))
          (if (<= (`KismetMathLibrary.VSize` (- (`self.K2_GetActorLocation`) (`self.K2_GetActorLocation` _array_element_2))) (`self.visionRange`))
            (`BlueprintSetLibrary.Set_Add` (`self.unitsInVision`) _array_element_2) ; add every enemy unit in visionRange to set
          )))
      ;[1 1 1] Tell enemy units observed
      (if (== (`BlueprintSetLibrary.Set_Length` (`self.unitsInVision`)) 0)
        (set `local.unitsObservedString` (`KismetStringLibrary.Concat_StrStr` "No enemies observed within " (`KismetStringLibrary.Conv_IntToString` (`KismetMathLibrary.Round` (`self.visionRange`))) " cm."))
        (else
          (set `local.unitsObservedString` "Enemies observed: ")
          (bind _result (`BlueprintSetLibrary.Set_ToArray` (`self.unitsInVision`)))
          (for _array_element_3 _result
            (set `local.unitsObservedString` (`KismetStringLibrary.Concat_StrStr` (`local.unitsObservedString`) (`KismetSystemLibrary.GetDisplayName` _array_element_3) " " (`KismetStringLibrary.Conv_IntToString` (* (`KismetMathLibrary.Round` (/ (`KismetMathLibrary.VSize` (- (`self.K2_GetActorLocation`) (`self.K2_GetActorLocation` _array_element_3))) 5.0)) 5)) " cm " (`|GetArrayItem` (`self.compassDirections`) (`KismetMathLibrary.Round` (/ (+ (.yaw (`KismetMathLibrary.FindLookAtRotation` (`self.K2_GetActorLocation`) (`self.K2_GetActorLocation` _array_element_3))) 180.0) 45.0))) " of " "us. "))))))
    (:`then_3`
      (bind _output_get (set `self.lastRadioReport` (`KismetStringLibrary.Concat_StrStr` (`KismetSystemLibrary.GetDisplayName` self) " reporting:  \n" (`KismetStringLibrary.Concat_StrStr` (`KismetStringLibrary.Conv_IntToString` (* (`KismetMathLibrary.Round` (/ (`self.closestLandmarkDistance`) 5.0)) 5)) " cm " (`|GetArrayItem` (`self.compassDirections`) (`KismetMathLibrary.Round` (/ (+ (.yaw (`KismetMathLibrary.FindLookAtRotation` (`self.K2_GetActorLocation` (`self.closestLandmark`)) (`self.K2_GetActorLocation`))) 180.0) 45.0))) " of " (`/Game/Blueprint/Landmark.name` (`self.closestLandmark`)) ", in " (`self.currentTerrainName`) ". ") (`KismetStringLibrary.Concat_StrStr` "Moving towards " (`|GetArrayItem` (`self.compassDirections`) (`KismetMathLibrary.Round` (/ (+ (.yaw (`KismetMathLibrary.FindLookAtRotation` (`self.K2_GetActorLocation`) (`self.moveCommand`))) 180.0) 45.0))) ". ") (`KismetStringLibrary.Concat_StrStr` "Strength is " (`KismetStringLibrary.Conv_IntToString` (`KismetMathLibrary.Round` 0.0)) ". ") " \n" (`local.unitsObservedString`))))
      (`KismetArrayLibrary.Array_Append` (`self.radioReports`) (`|MakeArray` _output_get)))))

(fn `UserConstructionScript`)