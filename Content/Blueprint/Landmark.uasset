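; Landmark is a placeable actor that marks a named location in the level with a static mesh and a nametag widget.
; On BeginPlay it swaps in the optional MeshOverride mesh when one is set, so each instance can use its own model chosen in the editor.
; It then passes its Name to the LandmarkNametagHUD widget inside the NametagWidget component for display.
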(event `self.ReceiveBeginPlay`
  (`|ExecutionSequence`
    (:`then_0`
      ;[1 1 1] Can replace static mesh in editor
      (`/Engine/EditorBlueprintResources/StandardMacros.IsValid` (`self.meshOverride`)
        (:`Is Valid`
          (`StaticMeshComponent.SetStaticMesh` (`self.StaticMesh`) (`self.meshOverride`)))))
    (:`then_1`
      ;[1 1 1] Set the nametag widget to display the name of this Landmark
      (bind _aslandmark_nametag_hud (cast `/Game/UI/LandmarkNametagHUD` (`WidgetComponent.GetUserWidgetObject` (`self.nametagWidget`))))
      (set `/Game/UI/LandmarkNametagHUD.textNametag` (`self.name`) _aslandmark_nametag_hud))))

(fn `UserConstructionScript`)