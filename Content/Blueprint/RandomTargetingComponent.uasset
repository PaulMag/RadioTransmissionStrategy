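; An actor component that sends its owning Unit toward one randomly chosen player unit or city.
; On BeginPlay it builds a target set from Infantry, Cavalry and Armored units, matched by exact class, plus every City, then picks one at random.
; Each Tick writes that target's current location to the owner's MoveCommand, with no retargeting or validity check.
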(event `self.ReceiveBeginPlay`
  (`|ExecutionSequence`
    (:`then_0`
      ;[1 1 1] Empty set
      (set `self.targets` (`|MakeSet`)))
    (:`then_1`
      (bind _outactors (`GameplayStatics.GetAllActorsOfClass` "/Game/Blueprint/Unit.Unit_C"))
      (for _array_element _outactors
        (bind _returnvalue (`GameplayStatics.GetObjectClass` _array_element))
        ;[1 1 1] The player classes only
        (if (or (== _returnvalue "/Game/Blueprint/Infantry.Infantry_C") (== _returnvalue "/Game/Blueprint/Cavalry.Cavalry_C") (== _returnvalue "/Game/Blueprint/Armored.Armored_C"))
          (`BlueprintSetLibrary.Set_Add` (`self.targets`) _array_element))))
    (:`then_2`
      (bind _outactors_2 (`GameplayStatics.GetAllActorsOfClass` "/Game/Blueprint/City.City_C"))
      (for _array_element_2 _outactors_2
        (`BlueprintSetLibrary.Set_Add` (`self.targets`) _array_element_2)))
    (:`then_3`
      (bind _result (`BlueprintSetLibrary.Set_ToArray` (`self.targets`)))
      (set `self.target` (`|GetArrayItem` _result (`KismetMathLibrary.RandomInteger` (`KismetArrayLibrary.Array_Length` _result)))))))

(event `self.ReceiveTick`
  (params (DeltaSeconds :type "Float (single-precision)"))
  (bind _asunit (cast `/Game/Blueprint/Unit` (`self.GetOwner`)))
  (set `/Game/Blueprint/Unit.moveCommand` (`Actor.K2_GetActorLocation` (`self.target`)) _asunit))