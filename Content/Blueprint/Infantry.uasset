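; Infantry unit Blueprint that takes damage when another Unit overlaps it.
; On overlap it subtracts the other unit's damage points, scaled by its anti-infantry modifier, from its own hit points.
; The other unit's fortified state adds the damage-to-fortified modifier; otherwise, its marching state adds the marching modifier.
; Both fortified branches compute identical damage, and no death handling is present.
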(event `self.ReceiveActorBeginOverlap`
  (params (OtherActor :type "Actor Object Reference"))
  (bind _asunit (cast `/Game/Blueprint/Unit` OtherActor))
  (if (`/Game/Blueprint/Unit.bIsFortified` _asunit)
    (bind _bismarching (`/Game/Blueprint/Unit.bIsMarching` _asunit))
    (if _bismarching
      (bind _damagepoints (`/Game/Blueprint/Unit.damagePoints` _asunit))
      (bind _moddamagetofortified (`/Game/Blueprint/Unit.modDamageToFortified` _asunit))
      (bind _moddamagetoinfantry (`/Game/Blueprint/Unit.modDamageToInfantry` _asunit))
      (set `self.hitPoints` (- (`self.hitPoints`) (* _damagepoints (* _moddamagetofortified _moddamagetoinfantry))))
      (else
        (set `self.hitPoints` (- (`self.hitPoints`) (* _damagepoints (* _moddamagetoinfantry _moddamagetofortified))))))
    (elif _bismarching
      (set `self.hitPoints` (- (`self.hitPoints`) (* _damagepoints (* _moddamagetoinfantry (`/Game/Blueprint/Unit.modDamageWhileMarching` _asunit)))))
      (else
        (set `self.hitPoints` (- (`self.hitPoints`) (* _damagepoints _moddamagetoinfantry)))))))

(fn `UserConstructionScript`
  (`parent.UserConstructionScript`))