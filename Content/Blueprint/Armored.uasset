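; Armored combat unit that loses hit points while overlapping other units and destroys itself at zero.
; Tick scans all Units, walks each overlapped unit's own overlaps and, after faction checks, applies those units' damage, modified against armor, for marching and for outnumbering.
; The single-target, non-marching branch multiplies by DeltaSeconds twice, unlike the others.
; On destruction, it prints every Unit's hit points and damage for debugging.
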(event `self.ReceiveTick`
  (params (DeltaSeconds :type "Float (single-precision)"))
  (`parent.ReceiveTick` DeltaSeconds)
  (bind _outactors (`GameplayStatics.GetAllActorsOfClass` "/Game/Blueprint/Unit.Unit_C"))
  (for _array_element _outactors
    (if (`self.IsOverlappingActor` _array_element)
      (for _array_element_2 (`self.GetOverlappingActors` _array_element "/Game/Blueprint/Unit.Unit_C")
        (bind _asunit (cast `/Game/Blueprint/Unit` _array_element_2)
          (:`then`
            ;[1 1 1] Player Is Overlapping Enemies?
            (if (`self.bIsEnemy`)
              ;[1 1 1] Enemy Is Overlapping Players?
              (if (not (`/Game/Blueprint/Unit.bIsEnemy` _array_element))
                ;[1 1 1] Enemy Overlapping more than 1 player?
                (if (>= (+ (`KismetArrayLibrary.Array_Length` (`self.GetOverlappingActors` _array_element "/Game/Blueprint/InfantryPlayer.InfantryPlayer_C")) (`KismetArrayLibrary.Array_Length` (`self.GetOverlappingActors` _array_element "/Game/Blueprint/CavalryPlayer.CavalryPlayer_C")) (`KismetArrayLibrary.Array_Length` (`self.GetOverlappingActors` _array_element "/Game/Blueprint/ArmoredPlayer.ArmoredPlayer_C"))) 2)
                  ;[1 1 1] Multiple Targets
                  (if (`/Game/Blueprint/Unit.bIsMarching` _asunit) :!label _label
                    (bind _damagepoints (`/Game/Blueprint/Unit.damagePoints` _asunit))
                    (bind _moddamagetoarmored (`/Game/Blueprint/Unit.modDamageToArmored` _asunit))
                    (bind _moddamagewhileoutnumbered (`/Game/Blueprint/Unit.modDamageWhileOutnumbered` _asunit))
                    (bind _returnvalue (- (`self.hitPoints`) (* DeltaSeconds (* _damagepoints (* (* _moddamagetoarmored _moddamagewhileoutnumbered) (`/Game/Blueprint/Unit.modDamageWhileMarching` _asunit))))))
                    ;;[1 1 1] Self Not Fortified, Target Is Marching
                    (bind _output_get (set `self.hitPoints` _returnvalue))
                    (`KismetSystemLibrary.PrintString` (`KismetStringLibrary.Conv_DoubleToString` _returnvalue) false)
                    (`/Engine/EditorBlueprintResources/StandardMacros.CompareFloat` _output_get
                      (:`==`
                        _)
                      (:`<`
                        _))
                    (`self.K2_DestroyActor`)
                    (`KismetSystemLibrary.PrintString` "Unit Destroyed")
                    (else
                      (bind _returnvalue_2 (- (`self.hitPoints`) (* DeltaSeconds (* _damagepoints (* _moddamagetoarmored _moddamagewhileoutnumbered)))))
                      ;;[1 1 1] Self Not Fortified, Target Not Marching
                      (bind _output_get_2 (set `self.hitPoints` _returnvalue_2))
                      (`KismetSystemLibrary.PrintString` (`KismetStringLibrary.Conv_DoubleToString` _returnvalue_2) false)
                      (`/Engine/EditorBlueprintResources/StandardMacros.CompareFloat` _output_get_2
                        (:`==`
                          _)
                        (:`<`
                          _))
                      (`self.K2_DestroyActor`)
                      (`KismetSystemLibrary.PrintString` "Unit Destroyed")))
                  (else
                    ;[1 1 1] Single Target
                    (if (`/Game/Blueprint/Unit.bIsMarching` _asunit) :!label _label_2
                      (bind _damagepoints_2 (`/Game/Blueprint/Unit.damagePoints` _asunit))
                      (bind _moddamagetoarmored_2 (`/Game/Blueprint/Unit.modDamageToArmored` _asunit))
                      ;;[1 1 1] Self Not Fortified, Target Is Marching
                      (bind _output_get_3 (set `self.hitPoints` (- (`self.hitPoints`) (* (* _damagepoints_2 (* _moddamagetoarmored_2 (`/Game/Blueprint/Unit.modDamageWhileMarching` _asunit))) DeltaSeconds))))
                      (`KismetSystemLibrary.PrintString` (`KismetStringLibrary.Conv_DoubleToString` _output_get_3) false)
                      (`/Engine/EditorBlueprintResources/StandardMacros.CompareFloat` _output_get_3
                        (:`==`
                          _)
                        (:`<`
                          _))
                      (`self.K2_DestroyActor`)
                      (`KismetSystemLibrary.PrintString` "Unit Destroyed")
                      (else
                        ;;[1 1 1] Self Not Fortified, Target Not Marching
                        (bind _output_get_4 (set `self.hitPoints` (- (`self.hitPoints`) (* (* (* _damagepoints_2 _moddamagetoarmored_2) DeltaSeconds) DeltaSeconds))))
                        (`KismetSystemLibrary.PrintString` (`KismetStringLibrary.Conv_DoubleToString` _output_get_4) false)
                        (`/Engine/EditorBlueprintResources/StandardMacros.CompareFloat` _output_get_4
                          (:`==`
                            _)
                          (:`<`
                            _))
                        (`self.K2_DestroyActor`)
                        (`KismetSystemLibrary.PrintString` "Unit Destroyed"))))))
              (elif (`/Game/Blueprint/Unit.bIsEnemy` _asunit)
                ;[1 1 1] Player Overlapping more than 1 enemy?
                (if (>= (+ (`KismetArrayLibrary.Array_Length` (`self.GetOverlappingActors` _array_element "/Game/Blueprint/InfantryEnemy.InfantryEnemy_C")) (`KismetArrayLibrary.Array_Length` (`self.GetOverlappingActors` _array_element "/Game/Blueprint/ArmoredEnemy.ArmoredEnemy_C")) (`KismetArrayLibrary.Array_Length` (`self.GetOverlappingActors` _array_element "/Game/Blueprint/CavalryEnemy.CavalryEnemy_C"))) 2)
                  (goto _label)
                  (else
                    (goto _label_2))))))
          (:`CastFailed`
            (`KismetSystemLibrary.PrintString` "Casting failed!")))))))

(event `self.ReceiveDestroyed`
  (bind _outactors (`GameplayStatics.GetAllActorsOfClass` "/Game/Blueprint/Unit.Unit_C"))
  (for _array_element _outactors
    (`KismetSystemLibrary.PrintString` (`KismetStringLibrary.Conv_DoubleToString` (`/Game/Blueprint/Unit.hitPoints` _array_element)))
    (`KismetSystemLibrary.PrintString` (`KismetStringLibrary.Conv_DoubleToString` (`/Game/Blueprint/Unit.damagePoints` _array_element)))
    (bind _bisenemy (`/Game/Blueprint/Unit.bIsEnemy` _array_element))
    (`KismetSystemLibrary.PrintString` "Destroyed Was Enemy" _bisenemy _bisenemy)))

(fn `UserConstructionScript`
  (`parent.UserConstructionScript`))